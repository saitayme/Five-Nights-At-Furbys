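; BP_Item is an item that falls from a shelf (Regal) and can be picked up and put back with E.
; Its fall event hides the shelf's item and reveals the ground mesh.
; E inside the trigger copies the mesh to BP_DemoCharacter's HeldItem and shows the placement spot.
; While held, E places it via the shelf if the character overlaps any BP_Regal_Platz, tracked by the HaveFallen and IsHolding flags.
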(event `self.ReceiveBeginPlay`
  (`self.EnableInput` (`GameplayStatics.GetPlayerController` 0))
  (`StaticMeshComponent.SetStaticMesh` (`self.Item_On_Ground`) (`self.ItemRef`)))

(event `Key|E`
  (params (Key :type "Key Structure"))
  (:`Pressed`
    (if (`self.isHolding`)
      (bind _outactors (`GameplayStatics.GetAllActorsOfClass` "/Game/Dave_Ordner/BP_Regal_Platz.BP_Regal_Platz_C"))
      (for _array_element _outactors
        (bind _returnvalue (`GameplayStatics.GetActorOfClass` "/Game/Blueprints/BP_DemoCharacter.BP_DemoCharacter_C"))
        (if (`KismetArrayLibrary.Array_Contains` (`self.GetOverlappingActors` _array_element null) _returnvalue)
          (`/Game/Dave_Ordner/BP_Regal_Platz.Platziere` (`self.Regal`))
          (`StaticMeshComponent.SetStaticMesh` (`/Game/Blueprints/BP_DemoCharacter.HeldItem` _returnvalue) null)
          (set `self.isHolding` false)))
      (elif (`self.haveFallen`)
        (bind _returnvalue_2 (`GameplayStatics.GetActorOfClass` "/Game/Blueprints/BP_DemoCharacter.BP_DemoCharacter_C"))
        (if (`KismetArrayLibrary.Array_Contains` (`PrimitiveComponent.GetOverlappingActors` (`self.Trigger`) "/Game/Blueprints/BP_DemoCharacter.BP_DemoCharacter_C") _returnvalue_2)
          (`StaticMeshComponent.SetStaticMesh` (`/Game/Blueprints/BP_DemoCharacter.HeldItem` _returnvalue_2) (`self.ItemRef`))
          (`SceneComponent.SetVisibility` (`self.Item_On_Ground`) false false)
          (`/Game/Dave_Ordner/BP_Regal_Platz.Show Item Placement Spot` (`self.Regal`))
          (set `self.isHolding` true)
          (set `self.haveFallen` false))))))

(event `I have Fallen and I can't get up`
  (if (not (`self.haveFallen`))
    (`/Game/Dave_Ordner/BP_Regal_Platz.Hide Shelf Item` (`self.Regal`))
    (`SceneComponent.SetVisibility` (`self.Item_On_Ground`) true false)
    (set `self.haveFallen` true)))

(fn `UserConstructionScript`)